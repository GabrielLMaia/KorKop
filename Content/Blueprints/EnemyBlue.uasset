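; EnemyBlue is an enemy that chases the MainCharacter on sight and otherwise wanders to random nearby reachable points.
; Pawn sensing starts the chase, and See clears when the move succeeds or fails.
; Tick, throttled by a one-second Delay, drains player health by Damage times DeltaSeconds while overlapping.
; It is destroyed by Bullet overlap or by the player punching at close range.
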(event `self.PawnSensing.OnSeePawn`
  (params (Pawn :type "Pawn Object Reference"))
  (set `self.See` true)
  (bind _asmain_character (cast `/Game/Blueprints/MainCharacter` Pawn))
  (`|AIMoveTo` self (0.0 0.0 0.0) _asmain_character
    (:`OnSuccess`
      _)
    (:`OnFail`
      _))
  (set `self.See` false))

(event `self.ReceiveTick`
  (params (DeltaSeconds :type "Float (single-precision)"))
  (`KismetSystemLibrary.Delay` 1.0)
  (if (not (`self.See`))
    (`|AIMoveTo` self (`NavigationSystem.K2_GetRandomReachablePointInRadius` (`self.K2_GetActorLocation`) 250.0)
      (:`then`
        _)))
  (if (`self.Close`)
    (bind _asmain_character (cast `/Game/Blueprints/MainCharacter` (`GameplayStatics.GetPlayerPawn` 0)))
    (if (`/Game/Blueprints/MainCharacter.Punching` _asmain_character)
      (`self.K2_DestroyActor`)
      (else
        (set `/Game/Blueprints/MainCharacter.HealthPoints` (- (`/Game/Blueprints/MainCharacter.HealthPoints` _asmain_character) (* DeltaSeconds (`self.Damage`))) _asmain_character)))))

(event `self.ReceiveActorBeginOverlap`
  (params (OtherActor :type "Actor Object Reference"))
  (cast `/Game/Blueprints/MainCharacter` OtherActor
    (:`then`
      (set `self.Close` true))
    (:`CastFailed`
      (cast `/Game/Blueprints/Bullet` OtherActor)
      (`self.K2_DestroyActor`))))

(event `self.ReceiveActorEndOverlap`
  (params (OtherActor :type "Actor Object Reference"))
  (cast `/Game/Blueprints/MainCharacter` OtherActor)
  (set `self.Close` false))

(fn `Move`)

(fn `UserConstructionScript`)