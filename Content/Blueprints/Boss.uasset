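; Boss actor that turns to face the player and fires projectiles at them.
; Tick sets the skeletal mesh's yaw toward player pawn 0, with a 90-degree offset and zeroed pitch and roll.
; Any overlap with Boss_Area starts a looping one-second timer on Fire, with no stop logic.
; Fire spawns a Boss_Bullet at the Arrow component, rotated toward the player's current position.
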(event `self.Boss_Area.OnComponentBeginOverlap`
  (params (OverlappedComponent :type "PrimitiveComponent Object Reference") (OtherActor :type "Actor Object Reference") (OtherComp :type "PrimitiveComponent Object Reference") (OtherBodyIndex :type Integer) (bFromSweep :type Boolean) (SweepResult :type "HitResult Structure (by ref)"))
  (`KismetSystemLibrary.K2_SetTimer` null "Fire" 1.0 true))

(event `self.ReceiveTick`
  (params (DeltaSeconds :type "Float (single-precision)"))
  (bind (_returnvalue_roll _returnvalue_pitch _returnvalue_yaw) (`KismetMathLibrary.BreakRotator` (`KismetMathLibrary.FindLookAtRotation` (`SceneComponent.K2_GetComponentLocation` (`self.SkeletalMesh`)) (`self.K2_GetActorLocation` (`GameplayStatics.GetPlayerPawn` 0)))))
  (`SceneComponent.K2_SetWorldRotation` (`self.SkeletalMesh`) (`KismetMathLibrary.MakeRotator` 0.0 0.0 (- _returnvalue_yaw 90.0)) false false))

(fn `Fire`
  (bind _returnvalue (`SceneComponent.K2_GetComponentLocation` (`self.Arrow`)))
  (`|SpawnActorFromClass` "/Game/Blueprints/Boss_Bullet.Boss_Bullet_C" (`KismetMathLibrary.MakeTransform` _returnvalue (`KismetMathLibrary.FindLookAtRotation` _returnvalue (`self.K2_GetActorLocation` (`GameplayStatics.GetPlayerPawn` 0)))) "Undefined" "OverrideRootScale" null null))

(fn `UserConstructionScript`)